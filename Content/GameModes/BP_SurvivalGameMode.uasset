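; Survival game mode Blueprint that shows on-screen wave announcements as the wave state changes.
; On BeginPlay it binds to the game mode state-changed delegate and reacts to two states.
; Waiting for a new wave creates a countdown widget timed to the spawn wait, while spawning creates a plain text widget showing the current wave number.
; Wave state and spawning logic are not implemented in this graph.
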(event Custom|OnSurvivalGameModeStateChanged_Event
  (params (CurrentState :type EWarriorSurvivalGameModeState%20Enum :default "WaitSpawnNewWave"))
  (switch Utilities|FlowControl|Switch|SwitchonEWarriorSurvivalGameModeState CurrentState
    (:WaitSpawnNewWave
      (CallFunction|CreateWaveWidgetwithCountDown "New Wave Coming In" (Variables|Default|GetSpawnNewWaveWaitTime)))
    (:SpawningNeWWave
      (CallFunction|CreateWaveWidgetNoCountDown (Utilities|Text|FormatText "Wave {CurrentWaveCount}" (Variables|Default|GetCurrentWaveCount))))))

(event EventBeginPlay
  (EventDispatchers|AssignOnSurvivalGameModeStateChanged (delegate Custom|OnSurvivalGameModeStateChanged_Event)))

(event EventTick
  (params (DeltaSeconds :type Float%20%28single-precision%29)))

(fn ConstructionScript)

(fn CreateWaveWidgetwithCountDown
  (params (TextContentToDisplay :type Text) (InTotalCountDownTime :type Float%20%28double-precision%29))
  (bind _returnvalue (UserInterface|CreateWidget "/Game/Widgets/GameplayWidgets/WBP_WaveTextWithCountDown.WBP_WaveTextWithCountDown_C"))
  (UserInterface|Viewport|AddtoViewport _returnvalue 0)
  (Rendering|Components|TextRender|SetText (Variables|/Game/Widgets/GameplayWidgets/WBP_WaveTextWithCountDown.WBP_WaveTextWithCountDown_C|GetTextBlock_WaveText _returnvalue) TextContentToDisplay)
  (Default|StartCountDown _returnvalue InTotalCountDownTime))

(fn CreateWaveWidgetNoCountDown
  (params (TextContentToDisplay :type Text))
  (bind _returnvalue (UserInterface|CreateWidget "/Game/Widgets/GameplayWidgets/WBP_WaveTextNoCountDown.WBP_WaveTextNoCountDown_C"))
  (UserInterface|Viewport|AddtoViewport _returnvalue 0)
  (Rendering|Components|TextRender|SetText (Variables|/Game/Widgets/GameplayWidgets/WBP_WaveTextNoCountDown.WBP_WaveTextNoCountDown_C|GetTextBlock_WaveText _returnvalue) TextContentToDisplay))